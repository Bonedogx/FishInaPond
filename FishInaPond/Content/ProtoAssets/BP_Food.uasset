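; BP_Food is a pickup that grants the player an extra dash on overlap, with a limited number of uses.
; Each Sphere overlap by the player pawn calls AddOneDash on BP_ThirdPersonCharacter and decrements ByOverlappedtimes.
; The counter is checked before the actor filter, so once it is zero, the next overlap by any actor destroys the food without granting a dash.
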(event OnComponentBeginOverlap(Sphere)
  (params (OverlappedComponent :type Primitive%20Component%20Object%20Reference) (OtherActor :type Actor%20Object%20Reference) (OtherComp :type Primitive%20Component%20Object%20Reference) (OtherBodyIndex :type Integer) (bFromSweep :type Boolean) (SweepResult :type Hit%20Result%20Structure%20%28by%20ref%29))
  (bind _returnvalue (Game|Player|GetPlayerPawn 0))
  (if (== (Variables|Default|GetByOverlappedtimes) 0)
    (Actor|DestroyActor)
    (elif (== OtherActor _returnvalue)
      (bind _asbp_third_person_character (Utilities|Casting|CastToBP_ThirdPersonCharacter _returnvalue))
      (Default|AddOneDash _asbp_third_person_character)
      (bind _result (Math|Integer|DecrementInt (Variables|Default|GetByOverlappedtimes))
        (:%20%20
          (Variables|Default|SetByOverlappedtimes _result))))))

(event EventBeginPlay)

(event Collision|EventActorBeginOverlap
  (params (OtherActor :type Actor%20Object%20Reference)))

(event EventTick
  (params (DeltaSeconds :type Float%20%28single-precision%29)))

(fn ConstructionScript)