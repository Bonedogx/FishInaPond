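; Player health component that tracks its owner's health and raises damage and death dispatchers.
; BeginPlay fills health to maximum and adds a screen-space WBP_UI widget above the owner, passing it the health and owning actor.
; The any-damage handler truncates damage to an integer, passes it to DecreaseHealth and prints it in red.
; DecreaseHealth subtracts it, calls OnDamageTaken, then OnDeath at zero or below.
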(event Custom|OnTakeAnyDamage_Event
  (params (DamagedActor :type Actor%20Object%20Reference) (Damage :type Float%20%28single-precision%29) (DamageType :type Damage%20Type%20Object%20Reference) (InstigatedBy :type Controller%20Object%20Reference) (DamageCauser :type Actor%20Object%20Reference))
  (bind _returnvalue (Math|Float|Truncate Damage))
  (EventDispatchers|AssignOnTakeAnyDamage (Components|GetOwner) (delegate Custom|OnTakeAnyDamage_Event))
  (CallFunction|DecreaseHealth _returnvalue)
  (Development|PrintString (Utilities|String|ToString(Integer) _returnvalue) true true "(R=1.000000,G=0.018804,B=0.000000,A=1.000000)"))

(event EventBeginPlay
  ;[0.15 0.15 0.15 0.5] Widget Component: Input: Get widget comonponent from owner | Output Set widget to owners health
  ;;[0.15 0 0 0.5] Sets health at the begining
  (Variables|Default|SetCurrentHealth (Variables|Default|GetMaxHealth))
  ;;[0.15 0.15 0.15 0.5] Creates Widget on top of the player character
  (bind _returnvalue (Game|AddComponentbyClass (Components|GetOwner) "/Script/UMG.WidgetComponent" false (Math|Transform|MakeTransform "0.000000,0.000000,100.000000" "0, 0, 0" "1.000000,1.000000,1.000000")))
  (Class|WidgetComponent|SetDrawSize _returnvalue "(X=150.000000,Y=10.000000)")
  (Class|WidgetComponent|SetWidgetSpace _returnvalue "Screen")
  (Collision|SetCollisionEnabled _returnvalue "NoCollision")
  (bind _returnvalue_2 (UserInterface|CreateWidget "/Game/UI/WBP_UI.WBP_UI_C" 0 (Variables|Default|GetCurrentHealth) (Components|GetOwner)))
  (UserInterface|SetWidget _returnvalue _returnvalue_2))

(fn DecreaseHealth
  (params (Damage :type Integer))
  ;[0.15 0.15 0.15 0.5] DecreasedHealth| Input: call on function from any damage taken event | Output: Removes one point of damage
  (bind _output_get (Variables|Default|SetCurrentHealth (- (Variables|Default|GetCurrentHealth) Damage)))
  (Default|CallOnDamageTaken)
  (if (<= _output_get 0)
    (Default|CallOnDeath)))