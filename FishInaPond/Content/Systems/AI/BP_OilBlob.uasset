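; BP_OilBlob is an AI enemy that damages the player when they enter its sphere.
; It spawns its default controller and, after a short delay, runs BT_OilBlob.
; Unless BeingPulled is set, perception updates feed the blackboard with the player as TargetActor, or their last known location when sight is lost.
; Overlap between its capsule and a BP_Drone's capsule has the drone destroy the blob.
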(event OnTargetPerceptionUpdated(AIPerception)
  (params (Actor :type Actor%20Object%20Reference) (Stimulus :type AI%20Stimulus%20Structure))
  (bind _returnvalue (AI|GetBlackboard 0))
  ;[0.15 0.15 0.15 0.5] Update BB_OilBlob data for use in BT_OilBlob
  (if (Utilities|IsValid _returnvalue)
    (if (not (ScalableFloat|GetValueasBool _returnvalue (Utilities|Name|MakeLiteralName "BeingPulled")))
      (CallFunction|HandleSightSense Actor Stimulus))))

(event OnComponentBeginOverlap(CapsuleComponent)
  (params (OverlappedComponent :type Primitive%20Component%20Object%20Reference) (OtherActor :type Actor%20Object%20Reference) (OtherComp :type Primitive%20Component%20Object%20Reference) (OtherBodyIndex :type Integer) (bFromSweep :type Boolean) (SweepResult :type Hit%20Result%20Structure%20%28by%20ref%29))
  ;[0.15 0.15 0.15 0.5] Tell Drone to destroy this blob when this
  (bind _asbp_drone (Utilities|Casting|CastToBP_Drone OtherActor))
  (Utilities|Casting|CastToCapsuleComponent OtherComp)
  (Default|DestroyOilBlob _asbp_drone self))

(event OnComponentBeginOverlap(Sphere)
  (params (OverlappedComponent :type Primitive%20Component%20Object%20Reference) (OtherActor :type Actor%20Object%20Reference) (OtherComp :type Primitive%20Component%20Object%20Reference) (OtherBodyIndex :type Integer) (bFromSweep :type Boolean) (SweepResult :type Hit%20Result%20Structure%20%28by%20ref%29))
  (bind _returnvalue (Game|GetPlayerCharacter 0))
  (if (== OtherActor _returnvalue)
    (Game|Damage|ApplyDamage _returnvalue 1.0 0 self)))

(event EventBeginPlay
  (bind _self self)
  ;[0.15 0.15 0.15 0.5] Tell actor to use BT_OilBlob AI
  (Utilities|FlowControl|Sequence
    (:then_0
      (Pawn|SpawnDefaultController _self)
      (Utilities|FlowControl|Delay 1.5)
      (AI|RunBehaviorTree (AI|GetAIController _self) "/Game/Systems/AI/BT_OilBlob.BT_OilBlob"))))

(fn ConstructionScript)

(fn HandleSightSense
  (params (Actor :type Actor%20Object%20Reference) (Stimulus :type AI%20Stimulus%20Structure))
  (bind (_age _expirationage _strength _stimuluslocation _receiverlocation _tag _bsuccessfullysensed) (Utilities|Struct|BreakAIStimulus Stimulus))
  (bind _returnvalue (Game|GetPlayerCharacter 0))
  (bind _returnvalue_2 (AI|GetBlackboard 0))
  ;[0.15 0.15 0.15 0.5] Handle Sight: Uses AIPerception to see the player, then sets the values in BB_OilBlob for use in AI.
  (if (== Actor _returnvalue)
    (if (Utilities|IsValid _returnvalue_2)
      (AI|Components|Blackboard|SetValueasObject _returnvalue_2 (Utilities|Name|MakeLiteralName "TargetActor") (Utilities|SelectObject _returnvalue 0 _bsuccessfullysensed))
      (if (not _bsuccessfullysensed)
        (AI|Components|Blackboard|SetValueasVector (AI|GetBlackboard 0) (Utilities|Name|MakeLiteralName "LastKnownLocation") _stimuluslocation)
        (AI|Components|Blackboard|SetValueasBool (AI|GetBlackboard 0) (Utilities|Name|MakeLiteralName "RemembersLastKnown") true))
      (else
        (return)))
    (else
      (return))))