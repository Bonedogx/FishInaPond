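; Drone spawn zone that starts a timer when the player overlaps its box and spawns a batch of drones once.
; Tick shows the timer on the player's health component and, when time is at or below the threshold, scatters drones around DroneSpawnArea and stops the timer.
; BeginPlay briefly shifts the box away and back so a player spawning inside still triggers it.
; The construction script draws the spawn radius as a debug circle.
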(event OnComponentBeginOverlap(Box)
  (params (OverlappedComponent :type Primitive%20Component%20Object%20Reference) (OtherActor :type Actor%20Object%20Reference) (OtherComp :type Primitive%20Component%20Object%20Reference) (OtherBodyIndex :type Integer) (bFromSweep :type Boolean) (SweepResult :type Hit%20Result%20Structure%20%28by%20ref%29))
  ;[0.15 0.15 0.15 0.5] Start drone spawn timer when player enters zone for the first time.
  (Utilities|Casting|CastToBP_ThirdPersonCharacter OtherActor)
  (Default|StartTimer (Variables|Default|GetBP_DroneTimer)))

(event EventBeginPlay
  ;[0.15 0.15 0.15 0.5] Shifts hitbox so that, if the player spawns in the hitbox, the timer will still activate. (mostly for lvl1)
  (Transformation|AddWorldOffset (Variables|Default|GetBox) "0.000000,0.000000,10000.000000" false true)
  (Utilities|FlowControl|Delay 0.1)
  (Transformation|AddWorldOffset (Variables|Default|GetBox) "0.000000,0.000000,-10000.000000" false true))

(event EventTick
  (params (DeltaSeconds :type Float%20%28single-precision%29))
  (bind _bp_dronetimer (Variables|Default|GetBP_DroneTimer))
  (bind _time (Variables|/Game/Systems/AI/BP_DroneTimer.BP_DroneTimer_C|GetTime _bp_dronetimer))
  ;[0.15 0.15 0.15 0.5] Check timer every second. If it is above TimeForDrones, it will spawn drones once.
  (Default|SetTimerTextF (Actor|GetComponentbyClass (Game|Player|GetPlayerPawn 0) "/Game/Player/Blueprints/BP_PlayerHealth.BP_PlayerHealth_C") (Utilities|Text|ToText(Float) _time "HalfToEven"))
  (Utilities|FlowControl|Delay 1.0)
  (if (<= _time (Variables|Default|GetTimeForDrones))
    (Utilities|FlowControl|DoOnce false
      (:Completed
        (for _index (range 0 (Variables|Default|GetNumberOfDrones))
          (CallFunction|SpawnDrones))
        (Variables|/Game/Systems/AI/BP_DroneTimer.BP_DroneTimer_C|SetTimerStart? (Variables|Default|GetBP_DroneTimer) false)))))

(fn ConstructionScript
  (Rendering|Debug|FlushPersistentDebugLines)
  (Rendering|Debug|DrawDebugCircle (Transformation|GetWorldLocation (Variables|Default|GetDroneSpawnArea)) (Math|Conversions|ToFloat(Integer) (Variables|Default|GetSpawnRadius)) 16 "(R=1.000000,G=1.000000,B=1.000000,A=1.000000)" 999.0 0.0 "1.000000,0.000000,0.000000" "0.000000,1.000000,0.000000"))

(fn SpawnDrones
  ;[0.15 0.15 0.15 0.5] Generate a random location in a circle around DroneSpawnArea, then spawn a Drone there. Repeat for NumberOfDrones
  (Game|SpawnActorfromClass "/Game/Systems/AI/BP_Drone.BP_Drone_C" (Math|Transform|MakeTransform (+ (Transformation|GetWorldLocation (Variables|Default|GetDroneSpawnArea)) (* (* (Math|Random|RandomUnitVector) "1.000000,1.000000,0.000000") (Variables|Default|GetSpawnRadius))) "0, 0, 0" "1.000000,1.000000,1.000000") "AdjustIfPossibleButAlwaysSpawn" "MultiplyWithRoot" 0 0))