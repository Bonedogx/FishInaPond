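; Oil blob launcher that spawns a single BP_OilBlob when play begins and sends it flying.
; The blob spawns at the Cylinder's location, facing the Arrow's forward direction plus a small random, positive-only offset on each axis.
; Its CharacterMovement velocity is then set directly along that facing at a fixed speed.
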(event EventBeginPlay
  (CallFunction|SpawnOilBlob))

(fn ConstructionScript)

(fn SpawnOilBlob
  (bind _returnvalue (Game|SpawnActorfromClass "/Game/Systems/AI/BP_OilBlob.BP_OilBlob_C" (Math|Transform|MakeTransform (Transformation|GetWorldLocation (Variables|Default|GetCylinder)) (Math|Rotator|MakeRotationfromAxes (+ (Math|Rotator|GetRotationXVector (Transformation|GetWorldRotation (Variables|Default|GetArrow))) (Math|Vector|MakeVector (Math|Random|RandomFloatinRange 0.0 0.25) (Math|Random|RandomFloatinRange 0.0 0.25) (Math|Random|RandomFloatinRange 0.0 0.25))) "0, 0, 0" "0, 0, 0") "1.000000,1.000000,1.000000") "AdjustIfPossibleButAlwaysSpawn" "MultiplyWithRoot" 0 0))
  (Variables|/Script/Engine.MovementComponent|SetVelocity (Variables|/Script/Engine.Character|GetCharacterMovement _returnvalue) (* (Math|Vector|GetForwardVector (Variables|/Script/Engine.Actor|GetRootComponent _returnvalue)) 1000)))