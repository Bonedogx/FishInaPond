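; DamagComponent is an unfinished contact-damage component, marked as not in use and possibly kept for later.
; Its OnContactDamage event is empty, and the damage logic is disconnected, so it never runs.
; That logic sphere-traces from the owner, ignoring it, and deals damage to a hit actor's BP_PlayerHealth component.
; The trace end divides the owner's location by its scaled forward vector instead of offsetting it.
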(event Custom|OnContactDamage
  ;[0.15 0.15 0.15 0.5] NOT IN USE MAY USE LATER
)